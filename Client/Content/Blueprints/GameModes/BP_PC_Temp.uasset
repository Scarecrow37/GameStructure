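; BP_PC_Temp is a temporary player controller that shows a login screen when play begins.
; BeginPlay shows the mouse cursor, creates a WBP_LoginPanel widget, switches input to UI-only focused on it and adds it to the viewport.
; The controller binds to the panel's OnLoginRequested event, and its handler only prints the submitted ID and password, with no authentication.
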(event `self.ReceiveBeginPlay`
  (`|ExecutionSequence`
    (:`then_0`
      (set `self.bShowMouseCursor` true))
    (:`then_1`
      (bind _returnvalue (`|CreateWidget` "/Game/UMG/WBP_LoginPanel.WBP_LoginPanel_C"))
      (set `self.LoginWIdgetReference` _returnvalue))
    (:`then_2`
      (add `LoginPanel.OnLoginRequested` (`self.LoginWIdgetReference`) (delegate `Event LoginRequested`)))
    (:`then_3`
      (`WidgetBlueprintLibrary.SetInputMode_UIOnlyEx` self (`self.LoginWIdgetReference`)))
    (:`then_4`
      (`UserWidget.AddToViewport` (`self.LoginWIdgetReference`) 0))))

(event `Event LoginRequested`
  (params (ID :type "Text (by ref)") (Password :type "Text (by ref)"))
  (`|ExecutionSequence`
    (:`then_0`
      (`KismetSystemLibrary.PrintText` ID true true (struct :`R` 1.0 :`G` 0.40689 :`B` 0.70956 :`A` 1.0)))
    (:`then_1`
      (`KismetSystemLibrary.PrintText` Password true true (struct :`R` 1.0 :`G` 0.40689 :`B` 0.70956 :`A` 1.0)))))

(fn `UserConstructionScript`)